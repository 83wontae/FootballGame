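; Game state Blueprint for the football mode that holds the Red and Blue goal counts.
; AddGoal takes a team and increments the opposing team's count, so Red adds to Blue and vice versa.
; Both counts use RepNotify, and each notify broadcasts the ChangeTeamScore dispatcher with both totals.
; The event graph and construction script are empty.
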(fn `AddGoal`
  (params (Team :type "/Game/Football/Datas/EN_Team Enum" :default "NewEnumerator0"))
  (switch `/Game/Football/Datas/EN_Team` Team
    (:`NewEnumerator1`
      (set `self.BlueGoal` (+ (`self.BlueGoal`) 1)))
    (:`NewEnumerator2`
      (set `self.RedGoal` (+ (`self.RedGoal`) 1)))))

(fn `OnRep_BlueGoal`
  (`self.EventDispatcher_ChangeTeamScore` (`self.RedGoal`) (`self.BlueGoal`)))

(fn `OnRep_RedGoal`
  (`self.EventDispatcher_ChangeTeamScore` (`self.RedGoal`) (`self.BlueGoal`)))

(fn `UserConstructionScript`)