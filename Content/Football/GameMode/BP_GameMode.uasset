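; BP_GameMode is the football game mode that puts each new player on a Red or Blue team.
; When a player starts, it runs the parent handler, then passes the chosen team to that player's BP_PlayerState through UpdateTeam.
; FindTeam tallies teams across all BP_PlayerState actors and returns Blue only when Red has more members, so ties go to Red.
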(event `self.HandleStartingNewPlayer`
  (params (NewPlayer :type "PlayerController Object Reference"))
  (`parent.HandleStartingNewPlayer` NewPlayer)
  (bind _asbp_player_state (cast `/Game/Football/GameMode/BP_PlayerState` (`Controller.PlayerState` NewPlayer)))
  (`/Game/Football/GameMode/BP_PlayerState.UpdateTeam` _asbp_player_state (`self.FindTeam`)))

(fn `FindTeam`
  (returns (Team :type "/Game/Football/Datas/EN_Team Enum"))
  (locals (RedCount :type Integer) (BlueCount :type Integer))
  (bind _outactors (`GameplayStatics.GetAllActorsOfClass` "/Game/Football/GameMode/BP_PlayerState.BP_PlayerState_C"))
  (for _array_element _outactors
    (switch `/Game/Football/Datas/EN_Team` (`/Game/Football/GameMode/BP_PlayerState.Team` _array_element)
      (:`NewEnumerator1`
        (`/Engine/EditorBlueprintResources/StandardMacros.IncrementInt` (`local.RedCount`)))
      (:`NewEnumerator2`
        (`/Engine/EditorBlueprintResources/StandardMacros.IncrementInt` (`local.BlueCount`)))))
  (if (> (`local.RedCount`) (`local.BlueCount`))
    (return "NewEnumerator2")
    (else
      (return "NewEnumerator1"))))

(fn `UserConstructionScript`)