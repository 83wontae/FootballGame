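; Game mode for a football match that assigns teams and drives the match through Ready, Play and End.
; New players join the team with fewer members (Red on a tie), and Ready starts once at least two player controllers exist.
; It binds to BP_GameState dispatchers for state changes and elapsed time, advancing phases on fixed time thresholds.
; When play ends, it tells every player state to update its result.
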(event `self.ReceiveBeginPlay`
  (bind _asbp_game_state (cast `/Game/Football/GameMode/Game/BP_GameState` (`GameplayStatics.GetGameState`)))
  (add `/Game/Football/GameMode/Game/BP_GameState.EventDispatcher_ChangeGameState` _asbp_game_state (`|CreateDelegate` :!event `EventChangeGameState`))
  (add `/Game/Football/GameMode/Game/BP_GameState.EventDispatcher_TotalDeltaSeconds` _asbp_game_state (`|CreateDelegate` :!event `EventTotalDeltaSeconds`)))

(event `self.HandleStartingNewPlayer`
  (params (NewPlayer :type "PlayerController Object Reference"))
  (`parent.HandleStartingNewPlayer` NewPlayer)
  ; Team 정하기
  (bind _asbp_player_state (cast `/Game/Football/GameMode/Game/BP_PlayerState` (`Controller.PlayerState` NewPlayer)))
  (`/Game/Football/GameMode/Game/BP_PlayerState.UpdateTeam` _asbp_player_state (`self.FindTeam`))
  ; Ready 상태 변경 처리
  (if (`self.CheckToReady`)
    (bind _asbp_game_state (cast `/Game/Football/GameMode/Game/BP_GameState` (`GameplayStatics.GetGameState`)))
    (`/Game/Football/GameMode/Game/BP_GameState.ChangeGameState` _asbp_game_state "NewEnumerator1")))

(fn `CheckToReady`
  (returns (IsCanReady :type Boolean))
  (bind _outactors (`GameplayStatics.GetAllActorsOfClass` "/Game/Football/GameMode/Game/BP_PlayerController.BP_PlayerController_C"))
  (return (>= (`KismetArrayLibrary.Array_Length` _outactors) 2)))

(fn `EventChangeGameState`
  (params (GameState :type "/Game/Football/Datas/EN_GameState Enum" :default "NewEnumerator0"))
  (bind _output_get (set `self.Game State` GameState))
  (`KismetSystemLibrary.PrintString` (`KismetStringLibrary.Concat_StrStr` "ChangeGameState : " (`|GetEnumeratorNameAsString` _output_get)) true true (struct :`G` 0.66 :`B` 1.0 :`A` 1.0) 60.0))

(fn `EventTotalDeltaSeconds`
  (params (TotalDeltaSeconds :type "Float (double-precision)"))
  (switch `/Game/Football/Datas/EN_GameState` (`self.Game State`)
    (:`NewEnumerator1`
      (if (> TotalDeltaSeconds 5.0)
        (bind _asbp_game_state (cast `/Game/Football/GameMode/Game/BP_GameState` (`GameplayStatics.GetGameState`)))
        (`/Game/Football/GameMode/Game/BP_GameState.ChangeGameState` _asbp_game_state "NewEnumerator2")))
    (:`NewEnumerator2`
      (if (> TotalDeltaSeconds 30.0)
        (bind _asbp_game_state_2 (cast `/Game/Football/GameMode/Game/BP_GameState` (`GameplayStatics.GetGameState`)))
        (`/Game/Football/GameMode/Game/BP_GameState.ChangeGameState` _asbp_game_state_2 "NewEnumerator3")
        (bind _outactors (`GameplayStatics.GetAllActorsOfClass` "/Game/Football/GameMode/Game/BP_PlayerState.BP_PlayerState_C"))
        (for _array_element _outactors
          (`/Game/Football/GameMode/Game/BP_PlayerState.UpdateResult` _array_element))))))

(fn `FindTeam`
  (returns (Team :type "/Game/Football/Datas/EN_Team Enum"))
  (locals (RedCount :type Integer) (BlueCount :type Integer))
  (bind _outactors (`GameplayStatics.GetAllActorsOfClass` "/Game/Football/GameMode/Game/BP_PlayerState.BP_PlayerState_C"))
  (for _array_element _outactors
    (switch `/Game/Football/Datas/EN_Team` (`/Game/Football/GameMode/Game/BP_PlayerState.Team` _array_element)
      (:`NewEnumerator1`
        (`/Engine/EditorBlueprintResources/StandardMacros.IncrementInt` (`local.RedCount`)))
      (:`NewEnumerator2`
        (`/Engine/EditorBlueprintResources/StandardMacros.IncrementInt` (`local.BlueCount`)))))
  (if (> (`local.RedCount`) (`local.BlueCount`))
    (return "NewEnumerator2")
    (else
      (return "NewEnumerator1"))))

(fn `UserConstructionScript`)