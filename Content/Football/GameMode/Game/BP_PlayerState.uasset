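; BP_PlayerState is the player state for the football game mode, holding each player's team, nickname and goal count.
; Simple setter functions change these values, and RepNotify handlers broadcast each change through event dispatchers.
; On BeginPlay it passes itself to the local player's BP_Hud via BindPlayerState, linking the replicated state to the HUD.
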(event `self.ReceiveBeginPlay`
  (bind _asbp_hud (cast `/Game/Football/GameMode/Game/BP_Hud` (`PlayerController.GetHUD` (`GameplayStatics.GetPlayerController` 0))))
  (`/Game/Football/GameMode/Game/BP_Hud.BindPlayerState` _asbp_hud self))

(fn `AddGoal`
  (set `self.Goal` (+ (`self.Goal`) 1)))

(fn `ChangeNickName`
  (params (NickName :type String))
  (set `self.NickName` NickName))

(fn `OnRep_Goal`
  (`self.EventDispatcher_UpdateGoal` (`self.Goal`)))

(fn `OnRep_NickName`
  (`self.EventDispatcher_ChangeNickName` (`self.NickName`)))

(fn `OnRep_Team`
  (`self.EventDispatcher_UpdateTeam` (`self.Team`)))

(fn `UpdateTeam`
  (params (Team :type "/Game/Football/Datas/EN_Team Enum" :default "NewEnumerator0"))
  (set `self.Team` Team))

(fn `UserConstructionScript`)