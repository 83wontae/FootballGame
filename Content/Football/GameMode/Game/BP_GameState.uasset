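; Football match game state that holds the Red and Blue scores, the current match phase and an elapsed-time counter.
; AddGoal credits the team opposite the one passed in.
; ChangeGameState sets the phase and zeroes the counter, which Tick accumulates only during Ready.
; RepNotify handlers on score, phase and time rebroadcast changes through event dispatchers.
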(event `self.ReceiveTick`
  (params (DeltaSeconds :type "Float (single-precision)"))
  (switch `/Game/Football/Datas/EN_GameState` (`self.GameState`)
    (:`NewEnumerator1`
      (`self.TickReady` DeltaSeconds))))

(fn `AddGoal`
  (params (Team :type "/Game/Football/Datas/EN_Team Enum" :default "NewEnumerator0"))
  (switch `/Game/Football/Datas/EN_Team` Team
    (:`NewEnumerator1`
      (set `self.BlueGoal` (+ (`self.BlueGoal`) 1)))
    (:`NewEnumerator2`
      (set `self.RedGoal` (+ (`self.RedGoal`) 1)))))

(fn `ChangeGameState`
  (params (GameState :type "/Game/Football/Datas/EN_GameState Enum" :default "NewEnumerator0"))
  (set `self.GameState` GameState)
  (set `self.TotalDeltaSeconds` 0.0))

(fn `OnRep_BlueGoal`
  (`self.EventDispatcher_ChangeTeamScore` (`self.RedGoal`) (`self.BlueGoal`)))

(fn `OnRep_GameState`
  (`self.EventDispatcher_ChangeGameState` (`self.GameState`)))

(fn `OnRep_RedGoal`
  (`self.EventDispatcher_ChangeTeamScore` (`self.RedGoal`) (`self.BlueGoal`)))

(fn `OnRep_TotalDeltaSeconds`
  (`self.EventDispatcher_TotalDeltaSeconds` (`self.TotalDeltaSeconds`)))

(fn `TickReady`
  (params (DeltaSeconds :type "Float (double-precision)"))
  (set `self.TotalDeltaSeconds` (+ DeltaSeconds (`self.TotalDeltaSeconds`))))

(fn `UserConstructionScript`)