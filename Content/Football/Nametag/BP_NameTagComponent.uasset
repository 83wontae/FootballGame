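; BP_NameTagComponent is a character component that shows a name tag with name, HP and SH readouts in the football game.
; On BeginPlay it creates a NameTag widget linked to itself, adds it to the viewport and initializes it with the owning Character of its attach parent.
; SetName, SetHp and SetSH forward values to the widget, which is removed on EndPlay.
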(event `self.ReceiveBeginPlay`
  (bind _returnvalue (`|CreateWidget` "/Game/Football/Nametag/NameTagWidget.NameTagWidget_C" null self))
  (bind _output_get (set `self.NameTag` _returnvalue))
  (`UserWidget.AddToViewport` _output_get 0)
  (bind _ascharacter (cast `Character` (`self.GetOwner` (`self.GetAttachParent`))))
  (`self.InitCharacter` _ascharacter))

(event `self.ReceiveEndPlay`
  (params (EndPlayReason :type "EEndPlayReason Enum" :default "Destroyed"))
  (`Widget.RemoveFromParent` (`self.NameTag`)))

(fn `InitCharacter`
  (params (Character :type "Character Object Reference"))
  (`/Game/Football/Nametag/NameTagWidget.InitCharacter` (`self.NameTag`) Character))

(fn `SetHp`
  (params (CurHp :type "Float (double-precision)") (MaxHp :type "Float (double-precision)"))
  (`/Game/Football/Nametag/NameTagWidget.SetHp` (`self.NameTag`) CurHp MaxHp))

(fn `SetName`
  (params (Name :type String))
  (`/Game/Football/Nametag/NameTagWidget.SetName` (`self.NameTag`) Name))

(fn `SetSH `
  (params (CurSH :type "Float (double-precision)") (MaxSH :type "Float (double-precision)"))
  (`/Game/Football/Nametag/NameTagWidget.SetSH` (`self.NameTag`) CurSH MaxSH))