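; BP_GoalPost is a team-owned football goal that records a goal when the ball enters it.
; On the server only, its Box overlap casts the other actor to BP_Ball and calls AddGoal on BP_GameState with the post's Team value.
; The construction script colors the GoalPost by setting its material according to Team (None, Red or Blue).
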(event `self.Box.OnComponentBeginOverlap`
  (params (OverlappedComponent :type "PrimitiveComponent Object Reference") (OtherActor :type "Actor Object Reference") (OtherComp :type "PrimitiveComponent Object Reference") (OtherBodyIndex :type Integer) (bFromSweep :type Boolean) (SweepResult :type "HitResult Structure (by ref)"))
  (`/Engine/EditorBlueprintResources/ActorMacros.Switch Has Authority`
    (:`Authority`
      (cast `/Game/Football/Blueprints/BP_Ball` OtherActor)
      (bind _asbp_game_state (cast `/Game/Football/GameMode/BP_GameState` (`GameplayStatics.GetGameState`)))
      (`/Game/Football/GameMode/BP_GameState.AddGoal` _asbp_game_state (`self.Team`)))))

(fn `UserConstructionScript`
  (bind _goalpost (`self.GoalPost`))
  (switch `/Game/Football/Datas/EN_Team` (`self.Team`)
    (:`NewEnumerator0`
      (`PrimitiveComponent.SetMaterial` (`self.GoalPost`) 0 "/Engine/EditorMaterials/WidgetMaterial.WidgetMaterial"))
    (:`NewEnumerator1`
      (`PrimitiveComponent.SetMaterial` _goalpost 0 "/Engine/EditorMaterials/WidgetMaterial_X.WidgetMaterial_X"))
    (:`NewEnumerator2`
      (`PrimitiveComponent.SetMaterial` _goalpost 0 "/Engine/EditorMaterials/WidgetMaterial_Z.WidgetMaterial_Z"))))